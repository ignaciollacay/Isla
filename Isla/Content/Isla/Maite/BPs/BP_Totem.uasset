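; BP_Totem is a totem actor whose static mesh floats along Z around its starting relative location.
; The construction script assigns the mesh from the Mesh variable.
; On BeginPlay it stores the mesh's relative location, then plays a timeline whose Flotación track, scaled by PositionOffset, drives the Z offset.
; A random start time of up to four seconds desynchronizes the motion between instances.
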(event `self.ReceiveBeginPlay`
  (bind _staticmesh (`self.StaticMesh`))
  (bind (_relative_location_x _relative_location_y _relative_location_z) (`KismetMathLibrary.BreakVector` (`self.Relative Location`)))
  (set `self.timeOffset` (`KismetMathLibrary.RandomFloatInRange` 0.0 4.0))
  (set `self.Relative Location` (`SceneComponent.RelativeLocation` _staticmesh))
  (`|ExecutionSequence`
    (:`then_0`
      (bind (_direction `_flotación`) (`Timeline|Timeline` :`NewTime` (`self.timeOffset`) :!via `SetNewTime` :!label _label)
        (:`Update`
          (`SceneComponent.K2_SetRelativeLocationAndRotation` _staticmesh (`KismetMathLibrary.MakeVector` _relative_location_x _relative_location_y (+ (* `_flotación` (`self.positionOffset`)) _relative_location_z)) (`KismetMathLibrary.MakeRotator` 0.0) false false))))
    (:`then_1`
      (goto _label))))

(fn `UserConstructionScript`
  (`StaticMeshComponent.SetStaticMesh` (`self.StaticMesh`) (`self.Mesh`)))