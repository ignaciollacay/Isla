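; Spline mesh Blueprint that repeats a chosen static mesh along its spline, with no active runtime logic.
; The construction script splits the spline into sections of SectionLength, optionally derived from actor Z scale, and adds a Z-forward spline mesh with configurable collision to each.
; Helper functions supply local endpoints and tangents clamped to section length.
; FullLengthMeshes omits the extra final section that otherwise covers the remainder.
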(fn `Get end pos/tangent`
  (params (Index :type Integer))
  (returns (Location :type "Vector Structure") (Tangent :type "Vector Structure"))
  (bind _spline (`self.Spline`))
  (bind _returnvalue (* (+ Index 1) (`self.Section Length`)))
  (return (`SplineComponent.GetLocationAtDistanceAlongSpline` _spline _returnvalue "Local") (`KismetMathLibrary.ClampVectorSize` (`SplineComponent.GetTangentAtDistanceAlongSpline` _spline _returnvalue "Local") 0.0 (`self.Section Length`))))

(fn `Get Start Pos/tangent`
  (params (Index :type Integer))
  (returns (Location :type "Vector Structure") (Tangent :type "Vector Structure"))
  (bind _spline (`self.Spline`))
  (bind _returnvalue (* Index (`self.Section Length`)))
  (return (`SplineComponent.GetLocationAtDistanceAlongSpline` _spline _returnvalue "Local") (`KismetMathLibrary.ClampVectorSize` (`SplineComponent.GetTangentAtDistanceAlongSpline` _spline _returnvalue "Local") 0.0 (`self.Section Length`))))

(fn `UserConstructionScript`
  (bind (_returnvalue_x _returnvalue_y _returnvalue_z) (`KismetMathLibrary.BreakVector` (`self.GetActorScale3D`)))
  (bind _loop_index (`self.Loop Index`))
  (if (`self.Allow Scaling`)
    (set `self.Section Length` (* _returnvalue_z 100.0)))
  (if (`self.Full Length Meshes?`)
    (for _index (range (`KismetMathLibrary.FTrunc` (/ (`SplineComponent.GetSplineLength` (`self.Spline`)) (`self.Section Length`))))
      (set `self.Loop Index` _index)
      (bind _returnvalue (`AddComponent|NODE_AddSplineMeshComponent-0` :!label _label))
      (`StaticMeshComponent.SetStaticMesh` _returnvalue (`self.Spline Mesh`))
      (`SplineMeshComponent.SetForwardAxis` _returnvalue "Z" true)
      (bind (_location _tangent) (`self.Get Start Pos/tangent` _loop_index))
      (bind (_location_2 _tangent_2) (`self.Get end pos/tangent` _loop_index))
      (`SplineMeshComponent.SetStartAndEnd` _returnvalue _location _tangent _location_2 _tangent_2 true)
      (`PrimitiveComponent.SetCollisionEnabled` _returnvalue (`self.Collision Type`)))
    (else
      (for _index_2 (range (+ (`KismetMathLibrary.FTrunc` (/ (`SplineComponent.GetSplineLength` (`self.Spline`)) (`self.Section Length`))) 1))
        (set `self.Loop Index` _index_2)
        (goto _label)))))